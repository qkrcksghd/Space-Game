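; BP_LongBeam is a player laser beam actor that handles the beam's visuals.
; Every tick it line-traces along its forward vector on the Visibility channel, then feeds the hit point, or the full-distance end when nothing blocks, into the Niagara beam's LaserEnd parameter.
; A second Niagara impact effect moves to the hit location and shows only on a blocking hit; both effects are tinted orange on BeginPlay.
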(event `self.ReceiveBeginPlay`
  (`FXSystemComponent.SetColorParameter` (`self.Niagara`) "Colour" (struct :`R` 1.0 :`G` 0.373369 :`A` 1.0))
  (`FXSystemComponent.SetColorParameter` (`self.NiagaraImpact`) "Colour" (struct :`R` 1.0 :`G` 0.373369 :`A` 1.0)))

(event `self.ReceiveTick`
  (params (DeltaSeconds :type "Float (single-precision)"))
  (bind _returnvalue (`self.K2_GetActorLocation`))
  (bind _niagaraimpact (`self.NiagaraImpact`))
  (bind _returnvalue_2 (+ _returnvalue (* (`self.GetActorForwardVector`) (`self.Distance`))))
  (set `self.TraceEnd` _returnvalue_2)
  (bind _outhit (`KismetSystemLibrary.LineTraceSingle` _returnvalue _returnvalue_2 "TraceTypeQuery1"))
  (set `self.bHit` (`GameplayStatics.BreakHitResult` _outhit))
  (set `self.HitLocation` (`.Location` (`GameplayStatics.BreakHitResult` _outhit)))
  (`FXSystemComponent.SetVectorParameter` (`self.Niagara`) "LaserEnd" (select `bool` (`self.bHit`) :`false` (`self.TraceEnd`) :`true` (`self.HitLocation`)))
  (`SceneComponent.SetVisibility` _niagaraimpact (`self.bHit`) false)
  (`SceneComponent.K2_SetWorldLocation` _niagaraimpact (`self.HitLocation`) false false))

(fn `UserConstructionScript`)