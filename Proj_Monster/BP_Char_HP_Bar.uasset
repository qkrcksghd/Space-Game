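; BP_Char_HP_Bar is an actor that displays a character's health bar through a widget component.
; On BeginPlay it gets the Char_HP_Bar user widget from HPBarComp and caches its progress bar.
; UpdateLocation moves the actor to a given position, and UpdateHPBar sets the bar's percent to current HP divided by max HP.
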(event `self.ReceiveBeginPlay`
  (bind _aschar_hp_bar (cast `/Game/Proj_Monster/Char_HP_Bar` (`WidgetComponent.GetUserWidgetObject` (`self.HP_Bar_Comp`))))
  (set `self.progressbar HP Bar` (`/Game/Proj_Monster/Char_HP_Bar.ProgressBar_49` _aschar_hp_bar)))

(fn `Update HP Bar`
  (params (HP :type "Float (double-precision)") (`MAX HP` :type "Float (double-precision)"))
  (`ProgressBar.SetPercent` (`self.progressbar HP Bar`) (/ HP `MAX HP`)))

(fn `Update Location`
  (params (Location :type "Vector Structure"))
  (`self.K2_SetActorLocation` Location))

(fn `UserConstructionScript`)