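; BP_Monster1 is a monster that chases the player and explodes on contact.
; Each Tick it moves a fixed step along the normalized direction to player 0, without delta-time scaling, applying that world-space vector as a local offset without sweep.
; When its Capsule begins overlapping the player, it spawns the Monster_explosion emitter at its own location and destroys itself.
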(event `self.ReceiveTick`
  (params (DeltaSeconds :type "Float (single-precision)"))
  ;[1 1 1] 플레이어를 따라오는 부분
  (bind _output_get (set `self.Target Player Location` (- (`self.K2_GetActorLocation` (`GameplayStatics.GetPlayerCharacter` 0)) (`self.K2_GetActorLocation`))))
  (`self.K2_AddActorLocalOffset` (* (`KismetMathLibrary.Normal` _output_get 10.0) (10.0 10.0 10.0))))

(event `self.Capsule.OnComponentBeginOverlap`
  (params (OverlappedComponent :type "PrimitiveComponent Object Reference") (OtherActor :type "Actor Object Reference") (OtherComp :type "PrimitiveComponent Object Reference") (OtherBodyIndex :type Integer) (bFromSweep :type Boolean) (SweepResult :type "HitResult Structure (by ref)"))
  ;[1 1 1] 플레이어와 오버랩되면 몬스터 위치에서 폭발 이펙트 나오고 삭제
  (if (== OtherActor (`GameplayStatics.GetPlayerCharacter` 0))
    (`GameplayStatics.SpawnEmitterAtLocation` "/Game/Proj_Monster/Effects/Monster_explosion.Monster_explosion" (`self.K2_GetActorLocation`) (struct) (1.5 1.5 1.5))
    (`self.K2_DestroyActor`)))

(fn `UserConstructionScript`)