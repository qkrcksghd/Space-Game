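; BP_Monster2 is a monster that turns toward the player and shoots while the player is inside its Box trigger.
; Box overlap events set IsOverlap, though any actor leaving clears it.
; Tick uses a one-second Delay as a fire-rate limiter before calling MakeBullet.
; MakeBullet snaps rotation toward the player, stores RotationToPlayer, and spawns BP_Bullet at the Cube's location without passing that rotation.
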(event `self.ReceiveTick`
  (params (DeltaSeconds :type "Float (single-precision)"))
  (if (`self.isOverlap`)
    (`KismetSystemLibrary.Delay` 1.0)
    (`self.MakeBullet`)))

(event `self.Box.OnComponentBeginOverlap`
  (params (OverlappedComponent :type "PrimitiveComponent Object Reference") (OtherActor :type "Actor Object Reference") (OtherComp :type "PrimitiveComponent Object Reference") (OtherBodyIndex :type Integer) (bFromSweep :type Boolean) (SweepResult :type "HitResult Structure (by ref)"))
  (if (== OtherActor (`GameplayStatics.GetPlayerCharacter` 0))
    (set `self.isOverlap` true)))

(event `self.Box.OnComponentEndOverlap`
  (params (OverlappedComponent :type "PrimitiveComponent Object Reference") (OtherActor :type "Actor Object Reference") (OtherComp :type "PrimitiveComponent Object Reference") (OtherBodyIndex :type Integer))
  (set `self.isOverlap` false))

(fn `MakeBullet`
  (bind _returnvalue (`KismetMathLibrary.FindLookAtRotation` (`self.K2_GetActorLocation`) (`self.K2_GetActorLocation` (`GameplayStatics.GetPlayerCharacter` 0))))
  (`self.K2_SetActorRotation` _returnvalue)
  (set `self.RotationToPlayer` _returnvalue)
  (`|SpawnActorFromClass` "/Game/Proj_Monster/BP_Bullet.BP_Bullet_C" (`KismetMathLibrary.Conv_VectorToTransform` (`SceneComponent.GetSocketLocation` (`self.Cube`) "None")) "Undefined" "OverrideRootScale" null null))

(fn `UserConstructionScript`)